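; Base Blueprint for crafting stations, which opens the crafting UI when the player character is close enough.
; CanOpenInterface compares the character's distance from the station root to an activation threshold and stores the result in CanOpen.
; If in range and no craft menu is open, it flags BP_Character as crafting, disables movement and calls AddWidgetToViewPort on the passed-in station reference.
; That event creates W_Craft for the first player controller and adds it to the viewport.
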(event Custom|addWidgetToViewPort
  (bind _returnvalue (UserInterface|CreateWidget "/Game/CraftSystem/W_Craft.W_Craft_C" (Game|GetPlayerController 0)))
  (UserInterface|Viewport|AddtoViewport _returnvalue 0))

(fn ConstructionScript)

(fn CanOpenInterface
  (params (BP_CraftReference :type BP%20BASE%20General%20Craft%20Object%20Reference))
  (bind _asbp_character (Utilities|Casting|CastToBP_Character (Game|GetPlayerCharacter 0)))
  (if (< (Math|Vector|Distance(Vector) (Transformation|GetWorldLocation (Variables|/Script/Engine.Actor|GetRootComponent _asbp_character)) (Transformation|GetWorldLocation (Variables|Default|GetDefaultSceneRoot))) (Variables|Default|GetDistanceToPermtActivation))
    (Variables|Default|SetCanOpen true)
    (else
      (Variables|Default|SetCanOpen false)))
  (if (Variables|Default|GetCanOpen)
    (if (not (Variables|/Game/Player/Blueprints/BP_Character.BP_Character_C|GetIsCraftOpen _asbp_character))
      (Variables|/Game/Player/Blueprints/BP_Character.BP_Character_C|SetIsCraftOpen _asbp_character true)
      (Variables|/Game/Player/Blueprints/BP_Character.BP_Character_C|SetcanMove _asbp_character false)
      (CallFunction|AddWidgettoViewPort BP_CraftReference))))