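; BP_Spawner populates a map with resource actors on BeginPlay, or restores items from that map's save.
; It loads BP_SaveGame using the GameInstance's MapName as slot, respawning saved items at stored positions if HadBeenSaved is set.
; Otherwise it scatters actors at random XY points, rerolling any closer than Offest to earlier spawns.
; The spacing check skips the latest spawn, and the InifiniteSecurity retry counter is never checked.
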(event EventBeginPlay
  (bind _asbp_general_instance (Utilities|Casting|CastToBP_GeneralInstance (Game|GetGameInstance)))
  (Development|PrintString (Variables|/Game/UI/Sauvergarde/BP/BP_GeneralInstance.BP_GeneralInstance_C|GetMapName _asbp_general_instance) true true "(R=0.094060,G=1.000000,B=0.000000,A=1.000000)" 102.0)
  (bind _returnvalue (SaveGame|LoadGamefromSlot (Variables|/Game/UI/Sauvergarde/BP/BP_GeneralInstance.BP_GeneralInstance_C|GetMapName _asbp_general_instance)))
  (bind _asbp_save_game (Utilities|Casting|CastToBP_SaveGame _returnvalue))
  (Development|PrintString (Utilities|String|Append "Had Already Spawn" (Utilities|String|ToString(Boolean) (Variables|/Game/UI/Sauvergarde/BP/BP_SaveGame.BP_SaveGame_C|GetHadBeenSaved _asbp_save_game))) true true "(R=0.000000,G=0.660000,B=1.000000,A=1.000000)" 1e+01)
  (if (Variables|/Game/UI/Sauvergarde/BP/BP_SaveGame.BP_SaveGame_C|GetHadBeenSaved _asbp_save_game)
    ;[1 0.1875 0] REspawn If Have already Existed
    (for (_array_element _array_index) (Variables|/Game/UI/Sauvergarde/BP/BP_SaveGame.BP_SaveGame_C|GetItemsInWorld _asbp_save_game)
      (Game|SpawnActorfromClass (Utilities|GetClass _array_element) (Math|Transform|MakeTransform (Utilities|Array|Get(acopy) (Variables|/Game/UI/Sauvergarde/BP/BP_SaveGame.BP_SaveGame_C|GetItemsPositions _asbp_save_game) _array_index) "0, 0, 0" "1,1,1") "Undefined" _array_element 0))
    (else
      (bind (_posxout _posyout) (CallFunction|GenerateRandomVector))
      (bind _output_get (Variables|Default|SetMemVector (Math|Vector|MakeVector _posxout _posyout 0.0)))
      (bind _returnvalue_2 (Game|SpawnActorfromClass (Variables|Parameters|GetClassRefActorToSpawn) (Math|Transform|MakeTransform _output_get "0, 0, 0" "1,1,1") "Undefined" 0 0))
      (Utilities|Array|Add (Variables|Default|GetRessources_Array) _returnvalue_2)
      ;[1 0 0.2109] While not as ressources as we want
      (while (< (Utilities|Array|Length (Variables|Default|GetRessources_Array)) (Variables|Parameters|GetRessourcesToSpawn))
        (bind (_posxout_2 _posyout_2) (CallFunction|GenerateRandomVector))
        (Variables|Default|SetMemVector (Math|Vector|MakeVector _posxout_2 _posyout_2 0.0))
        (Variables|Default|Setindex 0)
        (while (< (Variables|Default|Getindex) (- (Utilities|Array|Length (Variables|Default|GetRessources_Array)) 1))
          (if (> (Math|Vector|Distance(Vector) (Variables|Default|GetMemVector) (Transformation|GetWorldLocation (Variables|/Script/Engine.Actor|GetRootComponent (Utilities|Array|Get(acopy) (Variables|Default|GetRessources_Array) (Variables|Default|Getindex))))) (Variables|Parameters|GetOffest))
            (Math|Integer|IncrementInt (Variables|Default|Getindex)
              (:%20%20
                (if true
                  _)))
            (else
              (bind (_posxout_3 _posyout_3) (CallFunction|GenerateRandomVector))
              (Variables|Default|SetMemVector (Math|Vector|MakeVector _posxout_3 _posyout_3 0.0))
              (Variables|Default|Setindex 0)
              (Math|Integer|IncrementInt (Variables|Default|GetInifiniteSecurity)))))
        ;[0 1 0.1328] SpawnActor
        (bind _returnvalue_3 (Game|SpawnActorfromClass (Variables|Parameters|GetClassRefActorToSpawn) (Math|Transform|MakeTransform (Variables|Default|GetMemVector) "0, 0, 0" "1,1,1") "Undefined" 0 0))
        (Utilities|Array|Add (Variables|Default|GetRessources_Array) _returnvalue_3)))))

(fn ConstructionScript)

(fn GenerateRandomVector
  (bind _maxrangetospawn (Variables|Parameters|GetMaxRangeToSpawn))
  (LocalVariables|SetPosX (Math|Random|RandomFloatinRange 0.0 _maxrangetospawn))
  (LocalVariables|SetPosY (Math|Random|RandomFloatinRange 0.0 _maxrangetospawn))
  (return (LocalVariables|GetPosX) (LocalVariables|GetPosY)))