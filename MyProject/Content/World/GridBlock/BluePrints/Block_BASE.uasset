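; Base grid block actor that computes snapped placement positions from the cursor hit and flags overlaps.
; GetGridPos uses a 100-unit grid for Inside and Block selections.
; For Outside it uses a 50-unit XY grid, accepting only points off the 100-unit grid on one axis and rotating 90 degrees by axis.
; Collider overlaps print the other actor and set HitSomethings, while construction applies Mat to the cube.
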(event OnComponentBeginOverlap(Collider)
  (params (OverlappedComponent :type Primitive%20Component%20Object%20Reference) (OtherActor :type Actor%20Object%20Reference) (OtherComp :type Primitive%20Component%20Object%20Reference) (OtherBodyIndex :type Integer) (bFromSweep :type Boolean) (SweepResult :type Hit%20Result%20Structure%20%28by%20ref%29))
  (if (!= OtherActor self)
    (Development|PrintString (Utilities|GetDisplayName OtherActor))
    (Utilities|IsValid OtherActor
      (:Is%20Valid
        (Variables|Default|SetHitSomethings true))
      (:Is%20Not%20Valid
        (Variables|Default|SetHitSomethings false)))))

(event EventBeginPlay)

(event Collision|EventActorBeginOverlap
  (params (OtherActor :type Actor%20Object%20Reference)))

(event EventTick
  (params (DeltaSeconds :type Float%20%28single-precision%29)))

(fn ConstructionScript
  (Rendering|Material|SetMaterial (Variables|Default|GetCube) 0 (Variables|Default|GetMat)))

(fn GetGridPos
  (params (Selection :type TypeBlockEnum%20Enum :default "NewEnumerator0"))
  (bind _outsidepos (Utilities|GetOutsideGridPos))
  (switch Utilities|FlowControl|Switch|SwitchonTypeBlockEnum Selection
    (:NewEnumerator0
      (return (Utilities|GetMiddleGridPos) "0, 0, 0"))
    (:NewEnumerator1
      (if (and (!= (Math|Float|%(Float) (.x _outsidepos) 1e+02) 0.0) (== (Math|Float|%(Float) (.y _outsidepos) 1e+02) 0.0))
        (return (Math|Vector|MakeVector (.x _outsidepos) (.y _outsidepos) (.z _outsidepos)) "0, 0, 0")
        (elif (and (== (Math|Float|%(Float) (.x _outsidepos) 1e+02) 0.0) (!= (Math|Float|%(Float) (.y _outsidepos) 1e+02) 0.0))
          (return (Math|Vector|MakeVector (.x _outsidepos) (.y _outsidepos) (.z _outsidepos)) "0,90.000000, 0"))))
    (:NewEnumerator2
      (return (Utilities|GetMiddleGridPos) "0, 0, 0"))))