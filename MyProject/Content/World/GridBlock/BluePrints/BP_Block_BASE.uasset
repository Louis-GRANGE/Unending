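; Base actor for grid-snapped placeable blocks, applying its material to a cube on construction.
; GetGridPos snaps the cursor's trace hit to a 100-unit grid; Inside and Block selections stay unrotated.
; Outside selections compare the cursor's offsets within the cell, from a 10-unit rounded position, to pick a quarter-turn rotation.
; Collider overlaps with blocks of a different Type toggle a HitSomethings flag, with debug prints.
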(event OnComponentEndOverlap(Collider)
  (params (OverlappedComponent :type Primitive%20Component%20Object%20Reference) (OtherActor :type Actor%20Object%20Reference) (OtherComp :type Primitive%20Component%20Object%20Reference) (OtherBodyIndex :type Integer))
  (bind _asblock_base (Utilities|Casting|CastToBP_Block_BASE OtherActor))
  (if (!= (Variables|BP_Block_BASE_C|GetType _asblock_base) (Variables|Default|GetType))
    (Variables|Default|SetHitSomethings false)
    (Development|PrintString "No HIT")))

(event OnComponentBeginOverlap(Collider)
  (params (OverlappedComponent :type Primitive%20Component%20Object%20Reference) (OtherActor :type Actor%20Object%20Reference) (OtherComp :type Primitive%20Component%20Object%20Reference) (OtherBodyIndex :type Integer) (bFromSweep :type Boolean) (SweepResult :type Hit%20Result%20Structure%20%28by%20ref%29))
  (bind _asblock_base (Utilities|Casting|CastToBP_Block_BASE OtherActor))
  (if (!= (Variables|BP_Block_BASE_C|GetType _asblock_base) (Variables|Default|GetType))
    (Variables|Default|SetHitSomethings true)
    (Development|PrintString "HitsSomeThings")))

(event EventBeginPlay)

(event Collision|EventActorBeginOverlap
  (params (OtherActor :type Actor%20Object%20Reference)))

(event EventTick
  (params (DeltaSeconds :type Float%20%28single-precision%29)))

(fn ConstructionScript
  (Rendering|Material|SetMaterial (Variables|Default|GetCube) 0 (Variables|Default|GetMat)))

(fn GetGridPos
  (params (Selection :type Enum_TypeBlock%20Enum :default "NewEnumerator0"))
  (bind _tenpos (Utilities|GetTenDivPos))
  (bind _returnvalue (+ (.y _tenpos) 5e+01))
  (bind _returnvalue_2 (+ (.x _tenpos) 5e+01))
  (bind _returnvalue_3 (Math|Float|%(Float) _returnvalue 1e+02))
  (bind _returnvalue_4 (Math|Float|%(Float) _returnvalue_2 1e+02))
  (bind _returnvalue_5 (Math|Float|Absolute(Float) _returnvalue_3))
  (bind _returnvalue_6 (Math|Float|Absolute(Float) _returnvalue_4))
  (switch Utilities|FlowControl|Switch|SwitchonEnum_TypeBlock Selection
    (:NewEnumerator0
      (return (Utilities|GetMiddleGridPos) "0, 0, 0"))
    (:NewEnumerator1
      ;[0.9922 0 1] OutsidePos
      (if (< _returnvalue_6 5e+01)
        (if (> _returnvalue_6 _returnvalue_5)
          (return (Utilities|GetMiddleGridPos) "0,-90.000000,0.000000")
          (else
            (return (Utilities|GetMiddleGridPos) "0,180.000000,0.000000")))
        (elif (> _returnvalue_6 5e+01)
          (if (> _returnvalue_6 _returnvalue_5)
            (return (Utilities|GetMiddleGridPos) "0,0.000000,0.000000")
            (else
              (return (Utilities|GetMiddleGridPos) "0,90.000000,0.000000"))))))
    (:NewEnumerator2
      (return (Utilities|GetMiddleGridPos) "0, 0, 0"))))