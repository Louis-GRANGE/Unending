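; Player camera actor that becomes the view target at BeginPlay and enables the mouse cursor, click and hover events.
; Each tick it eases toward the BP_Character mesh when horizontally too far, otherwise toward its own XY plus OffsetCam at mesh-relative height.
; Its rotation is interpolated to keep looking at the mesh.
; Zoom and Dezoom step the offset's Z within camera-to-mesh distance limits.
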(event Custom|Zoom
  ;[0 0 0] Zoom/Dezoom
  (if (> (Math|Vector|Distance(Vector) (Transformation|GetWorldLocation (Variables|/Script/Engine.Character|GetMesh (.AsBP%20Character (Utilities|Casting|CastToBP_Character (Game|GetPlayerCharacter 0))))) (Transformation|GetWorldLocation (Variables|Default|GetCamera))) 1e+02)
    (Variables|Default|SetoffsetCam (Math|Vector|MakeVector (.x (Variables|Default|GetoffsetCam)) (.y (Variables|Default|GetoffsetCam)) (- (.z (Variables|Default|GetoffsetCam)) 1e+01)))))

(event Custom|Dezoom
  ;[0 0 0] Zoom/Dezoom
  (if (< (Math|Vector|Distance(Vector) (Transformation|GetWorldLocation (Variables|/Script/Engine.Character|GetMesh (.AsBP%20Character (Utilities|Casting|CastToBP_Character (Game|GetPlayerCharacter 0))))) (Transformation|GetWorldLocation (Variables|Default|GetCamera))) 1e+03)
    (Variables|Default|SetoffsetCam (Math|Vector|MakeVector (.x (Variables|Default|GetoffsetCam)) (.y (Variables|Default|GetoffsetCam)) (+ (.z (Variables|Default|GetoffsetCam)) 1e+01)))))

(event EventBeginPlay
  (bind _returnvalue (Game|GetPlayerController 0))
  (bind _returnvalue_2 (Game|GetPlayerController 0))
  (Variables|/Script/Engine.PlayerController|SetbShowMouseCursor _returnvalue true)
  (Game|Player|SetViewTargetwithBlend _returnvalue self 0.0 "VTBlend_Linear" 0.0 false)
  (Variables|/Script/Engine.PlayerController|SetbEnableMouseOverEvents _returnvalue_2 true)
  (Variables|/Script/Engine.PlayerController|SetbEnableClickEvents _returnvalue_2 true))

(event Collision|EventActorBeginOverlap
  (params (OtherActor :type Actor%20Object%20Reference)))

(event EventTick
  (params (DeltaSeconds :type Float%20%28single-precision%29))
  (bind _returnvalue (Game|GetPlayerCharacter 0))
  (bind _camera (Variables|Default|GetCamera))
  (bind _camera_2 (Variables|Default|GetCamera))
  (bind _returnvalue_2 (Transformation|GetWorldLocation _camera_2))
  (bind _returnvalue_3 (Transformation|GetWorldLocation _camera))
  (bind _asbp_character (Utilities|Casting|CastToBP_Character _returnvalue))
  (bind _mesh (Variables|/Script/Engine.Character|GetMesh _asbp_character))
  (bind _returnvalue_4 (Transformation|GetWorldLocation _mesh))
  (if (> (Math|Vector|Distance2D(Vector) _returnvalue_3 _returnvalue_4) 5e+02)
    (Transformation|SetWorldLocation (Variables|Default|GetCamera) (Math|Interpolation|VInterpTo _returnvalue_3 _returnvalue_4 (Utilities|Time|GetWorldDeltaSeconds) 2.5) false false)
    (else
      (Transformation|SetWorldLocation (Variables|Default|GetCamera) (Math|Interpolation|VInterpTo (Transformation|GetWorldLocation (Variables|Default|GetCamera)) (+ (+ (Math|Vector|MakeVector (.x _returnvalue_2) (.y _returnvalue_2) 0.0) (Variables|Default|GetoffsetCam)) (Math|Vector|MakeVector 0.0 0.0 (.z (Transformation|GetWorldLocation (Variables|/Script/Engine.Character|GetMesh (.AsBP%20Character (Utilities|Casting|CastToBP_Character (Game|GetPlayerCharacter 0)))))))) (Utilities|Time|GetWorldDeltaSeconds) 2.5) false false)))
  (Transformation|SetWorldRotation (Variables|Default|GetCamera) (Math|Interpolation|RInterpTo (Transformation|GetWorldRotation (Variables|Default|GetCamera)) (Math|Rotator|FindLookatRotation (Transformation|GetWorldLocation (Variables|Default|GetCamera)) _returnvalue_4) (Utilities|Time|GetWorldDeltaSeconds) 5.0) false false))

(fn ConstructionScript)