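; Player character with cursor-driven click-to-move, grid block building, inventory toggle and crafting-station interaction, viewed through a spawned BP_Camera with wheel zoom.
; Holding left click repeatedly re-issues the move unless Work has locked movement.
; A toggles build mode, cycling block type and showing a translucent grid-snapped preview updated on Tick.
; Right click places blocks after range, trace and overlap checks, and separately traces for craft interfaces.
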(event Custom|Work
  (Components|Activation|SetActive (Variables|Default|GetSmoke) true false)
  (Variables|Boolean|SetcanMove false))

(event Custom|EndWork
  (Components|Activation|SetActive (Variables|Default|GetSmoke) false false)
  (Variables|Boolean|SetcanMove true))

(event EventBeginPlay
  (Variables|/Script/Engine.CharacterMovementComponent|SetMaxStepHeight (Variables|Character|GetCharacterMovement) 1e+02)
  (bind _returnvalue (Game|SpawnActorfromClass "/Game/Player/Blueprints/BP_Camera.BP_Camera_C" (Math|Transform|MakeTransform (Transformation|GetWorldLocation (Variables|Character|GetMesh)) "0, 0, 0" "1,1,1") "Undefined" 0 0))
  (Variables|ObjectReference|SetCamera _returnvalue)
  (Components|Activation|SetActive (Variables|Default|GetSmoke) false false))

(event EventTick
  (params (DeltaSeconds :type Float%20%28single-precision%29))
  (bind _particule (Variables|Default|GetParticule))
  (bind _blockchoise (Variables|ObjectReference|GetBlockChoise))
  (bind _defaultsceneroot (Variables|/Game/World/GridBlock/BluePrints/BP_Block_BASE.BP_Block_BASE_C|GetDefaultSceneRoot (.actorblock _blockchoise)))
  (Utilities|FlowControl|Sequence
    (:then_0
      ;[0 0 0] AuraSpawnBlock
      (if (Variables|Boolean|GetBuildSystem)
        (Collision|SetCollisionEnabled (Variables|/Game/World/GridBlock/BluePrints/BP_Block_BASE.BP_Block_BASE_C|GetCube (.actorblock (Variables|ObjectReference|GetBlockChoise))) "NoCollision")
        (if (.bBlockingHit (Utilities|GetGridMovePos))
          (bind (_pos _rotation) (Default|GetGridPos (.actorblock _blockchoise) (.type _blockchoise)))
          (Transformation|SetWorldLocation _defaultsceneroot _pos false false)
          (Transformation|SetWorldRotation _defaultsceneroot _rotation false false))))
    (:then_1
      (if (> (Math|Vector|VectorLength (Transformation|GetVelocity (Game|GetPlayerCharacter 0))) 0.5)
        (Utilities|FlowControl|Delay 0.3)
        (Rendering|SetVisibility _particule true false)
        (else
          (Rendering|SetVisibility _particule false false))))))

(event Input|ActionEvents|InputActionOpenSaveMenu
  (params (Key :type Key%20Structure :default "None"))
  ;[1 0 0.2109] Ouverture et fermeture du menu de sauvegarde
)

(event Input|ActionEvents|InputActionOpenCloseInventory
  (params (Key :type Key%20Structure :default "None"))
  (bind _hudbp (Variables|HUD|GetHUDBP))
  (bind _inventoryhud (Variables|/Game/UI/Inventory/HUD_Main.HUD_Main_C|GetInventoryHUD _hudbp))
  ;[0 1 0.1328] Ouverture et fermeture de l'inventaire
  (:Pressed
    (Utilities|FlowControl|FlipFlop
      (:A
        (Default|OpenInventory _inventoryhud))
      (:B
        (Default|CloseInventory _inventoryhud)))))

(event Input|MouseEvents|LeftMouseButton
  (params (Key :type Key%20Structure :default "None"))
  (bind (_bblockinghit _returnvalue) (Utilities|GetGridMovePos))
  ;[0 0 0] MovePlayer
  (:Pressed
    (Utilities|FlowControl|Sequence
      (:then_0
        (goto _label Open))
      (:then_1
        (Utilities|FlowControl|Gate true :!label _label
          (:Exit
            (Utilities|FlowControl|Sequence
              (:then_0
                (if (Variables|Boolean|GetcanMove)
                  (if _bblockinghit
                    (AI|Navigation|SimpleMovetoLocation (Pawn|GetController) _returnvalue))))
              (:then_1
                (Utilities|FlowControl|RetriggerableDelay 0.12)
                (goto _label))))))))
  (:Released
    (goto _label Close)))

(event Input|KeyboardEvents|A
  (params (Key :type Key%20Structure :default "None"))
  ;[0 0 0] ChangeTypeBlock
  (:Pressed
    (bind _isa (Utilities|FlowControl|FlipFlop)
      (:A
        _)
      (:B
        _))
    (bind _output_get (Variables|Boolean|SetBuildSystem _isa))
    (if _output_get
      (switch int (Variables|Numbers|GetChangeBlock) :!label _label
        (:Default
          (Variables|Numbers|SetChangeBlock 0)
          (goto _label))
        (:0
          (Variables|ObjectReference|SetBlockChoise (Utilities|Struct|MakeStruct_BlockStruct "/Game/World/GridBlock/BluePrints/BP_Block_Black.BP_Block_Black_C" 0 "NewEnumerator1"))
          (Math|Integer|IncrementInt (Variables|Numbers|GetChangeBlock)
            (:%20%20
              _)))
        (:1
          (Variables|ObjectReference|SetBlockChoise (Utilities|Struct|MakeStruct_BlockStruct "/Game/World/GridBlock/BluePrints/BP_Block_Blue.BP_Block_Blue_C" 0 "NewEnumerator2"))
          (Math|Integer|IncrementInt (Variables|Numbers|GetChangeBlock)
            (:%20%20
              _)))
        (:2
          (Variables|ObjectReference|SetBlockChoise (Utilities|Struct|MakeStruct_BlockStruct "/Game/World/GridBlock/BluePrints/BP_Block_BASE.BP_Block_BASE_C" 0 "NewEnumerator2"))
          (Math|Integer|IncrementInt (Variables|Numbers|GetChangeBlock)
            (:%20%20
              _))))
      (bind _pos (Default|GetGridPos (.actorblock (Variables|ObjectReference|GetBlockChoise)) (.type (Variables|ObjectReference|GetBlockChoise))))
      (bind _returnvalue (Game|SpawnActorfromClass (.blockclass (Variables|ObjectReference|GetBlockChoise)) (Math|Conversions|ToTransform(Vector) _pos) "Undefined" 0 0))
      (bind _output_get_2 (Variables|ObjectReference|SetBlockChoise (Utilities|Struct|MakeStruct_BlockStruct (.blockclass (Variables|ObjectReference|GetBlockChoise)) _returnvalue (.type (Variables|ObjectReference|GetBlockChoise)))))
      (bind _returnvalue_2 (Rendering|Material|CreateDynamicMaterialInstance (Variables|/Game/World/GridBlock/BluePrints/BP_Block_BASE.BP_Block_BASE_C|GetMat (.actorblock _output_get_2)) "None" :!class /Script/Engine.KismetMaterialLibrary))
      (Rendering|Material|SetScalarParameterValue _returnvalue_2 "MyOpacity" 0.5 :!class /Script/Engine.MaterialInstanceDynamic)
      (Rendering|Material|SetMaterial (Variables|/Game/World/GridBlock/BluePrints/BP_Block_BASE.BP_Block_BASE_C|GetCube (.actorblock _output_get_2)) 0 _returnvalue_2)
      (else
        (Actor|DestroyActor (.actorblock (Variables|ObjectReference|GetBlockChoise)))))))

(event Input|MouseEvents|RightMouseButton
  (params (Key :type Key%20Structure :default "None"))
  (bind _blockchoise (Variables|ObjectReference|GetBlockChoise))
  (bind _mesh (Variables|Character|GetMesh))
  (bind _returnvalue (Transformation|GetWorldLocation _mesh))
  ;[0 0 0] Spawn Block
  (:Pressed
    (if (Variables|Boolean|GetBuildSystem)
      (bind (_pos _rotation) (Default|GetGridPos (.actorblock _blockchoise) (.type _blockchoise)))
      (if (<= (Math|Vector|Distance(Vector) _pos _returnvalue) (Variables|Numbers|GetDistanceToSpawnBlock))
        (bind _returnvalue_2 (Collision|LineTraceByChannel _returnvalue (Math|Vector|GetForwardVector (Math|Conversions|RotationFromXVector _pos)) "TraceTypeQuery1" false 0 "None"))
        (if _returnvalue_2
          (if (not (Variables|/Game/World/GridBlock/BluePrints/BP_Block_BASE.BP_Block_BASE_C|GetHitSomethings (.actorblock (Variables|ObjectReference|GetBlockChoise))))
            (Game|SpawnActorfromClass (.blockclass _blockchoise) (Math|Transform|MakeTransform _pos _rotation "1,1,1") "Undefined" 0 0)))))))

(event Input|MouseEvents|RightMouseButton
  (params (Key :type Key%20Structure :default "None"))
  (bind _returnvalue (Game|GetPlayerController 0))
  (bind (_worldlocation _worlddirection) (Game|Player|ConvertMouseLocationToWorldSpace _returnvalue))
  ;[0.2656 1 0] OUvertur et Fermeture des différentes interfaces de craft
  (:Pressed
    (bind _outhit (Collision|LineTraceByChannel _worldlocation (+ _worldlocation (* _worlddirection 1e+03)) "TraceTypeQuery1" false 0 "None"))
    (Development|PrintString (Utilities|GetDisplayName (.HitActor (Collision|BreakHitResult _outhit))))
    (bind _asbp_base_general_craft (Utilities|Casting|CastToBP_BASE_GeneralCraft (.HitActor (Collision|BreakHitResult _outhit))))
    (Default|CanOpenInterface _asbp_base_general_craft _asbp_base_general_craft)))

(event Input|MouseEvents|MouseWheelUp
  (params (Key :type Key%20Structure :default "None"))
  ;[0 0 0] Zoom/Dezoom
  (:Pressed
    (Default|Zoom (Variables|ObjectReference|GetCamera))))

(event Input|MouseEvents|MouseWheelDown
  (params (Key :type Key%20Structure :default "None"))
  ;[0 0 0] Zoom/Dezoom
  (:Pressed
    (Default|Dezoom (Variables|ObjectReference|GetCamera))))

(fn ConstructionScript)