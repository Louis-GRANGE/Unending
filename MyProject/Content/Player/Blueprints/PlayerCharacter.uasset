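; Player character with click-to-move, grid-based block building, a spawned zoomable camera and a toggled save menu.
; Holding left mouse repeats move orders through a gate and delay loop, which Work/EndWork suspend while showing smoke.
; A toggles build mode, cycling block type per activation and spawning a translucent preview that Tick snaps to the grid.
; Right click places the block after distance, line-trace and overlap checks.
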(event Custom|Work
  (Components|Activation|SetActive (Variables|Default|GetSmoke) true false)
  (Variables|Default|SetcanMove false))

(event Custom|EndWork
  (Components|Activation|SetActive (Variables|Default|GetSmoke) false false)
  (Variables|Default|SetcanMove true))

(event EventBeginPlay
  (Variables|/Script/Engine.CharacterMovementComponent|SetMaxStepHeight (Variables|Character|GetCharacterMovement) 1e+02)
  (bind _returnvalue (Game|SpawnActorfromClass "/Game/Player/Blueprints/Camera.Camera_C" (Math|Transform|MakeTransform (Transformation|GetWorldLocation (Variables|Default|GetCube)) "0, 0, 0" "1,1,1") "Undefined" 0 0))
  (Variables|Default|SetCamera _returnvalue)
  (Components|Activation|SetActive (Variables|Default|GetSmoke) false false))

(event EventTick
  (params (DeltaSeconds :type Float%20%28single-precision%29))
  (bind _blockchoise (Variables|Default|GetBlockChoise))
  (bind _defaultsceneroot (Variables|/Game/World/GridBlock/BluePrints/Block_BASE.Block_BASE_C|GetDefaultSceneRoot (.actorblock _blockchoise)))
  ;[0 0 0] AuraSpawnBlock
  (if (Variables|Default|GetBuildSystem)
    (Collision|SetCollisionEnabled (Variables|/Game/World/GridBlock/BluePrints/Block_BASE.Block_BASE_C|GetCube (.actorblock (Variables|Default|GetBlockChoise))) "NoCollision")
    (if (.bBlockingHit (Utilities|GetGridMovePos))
      (bind (_pos _rotation) (Default|GetGridPos (.actorblock _blockchoise) (.type _blockchoise)))
      (Transformation|SetWorldLocation _defaultsceneroot _pos false false)
      (Transformation|SetWorldRotation _defaultsceneroot _rotation false false))))

(event Input|ActionEvents|InputActionOpenSaveMenu
  (params (Key :type Key%20Structure :default "None"))
  (:Pressed
    (if (Variables|Default|GetisSaveMenuOpen)
      (Variables|Default|SetisSaveMenuOpen false)
      (Viewport|RemoveAllWidgets)
      (else
        (Variables|Default|SetisSaveMenuOpen true)
        (bind _returnvalue (UserInterface|CreateWidget "/Game/UI/Sauvergarde/Widgets/SaveMenu.SaveMenu_C"))
        (UserInterface|Viewport|AddtoViewport _returnvalue 0)))))

(event Input|MouseEvents|LeftMouseButton
  (params (Key :type Key%20Structure :default "None"))
  (bind (_bblockinghit _returnvalue) (Utilities|GetGridMovePos))
  ;[0 0 0] MovePlayer
  (:Pressed
    (Utilities|FlowControl|Sequence
      (:then_0
        (goto _label Open))
      (:then_1
        (Utilities|FlowControl|Gate true :!label _label
          (:Exit
            (Utilities|FlowControl|Sequence
              (:then_0
                (if (Variables|Default|GetcanMove)
                  (if _bblockinghit
                    (AI|Navigation|SimpleMovetoLocation (Pawn|GetController) _returnvalue))))
              (:then_1
                (Utilities|FlowControl|RetriggerableDelay 0.12)
                (goto _label))))))))
  (:Released
    (goto _label Close)))

(event Input|KeyboardEvents|A
  (params (Key :type Key%20Structure :default "None"))
  ;[0 0 0] ChangeTypeBlock
  (:Pressed
    (bind _isa (Utilities|FlowControl|FlipFlop)
      (:A
        _)
      (:B
        _))
    (bind _output_get (Variables|Default|SetBuildSystem _isa))
    (if _output_get
      (switch int (Variables|Default|GetChangeBlock) :!label _label
        (:Default
          (Variables|Default|SetChangeBlock 0)
          (goto _label))
        (:0
          (Variables|Default|SetBlockChoise (Utilities|Struct|MakeBlockStruct "/Game/World/GridBlock/BluePrints/Block_Black.Block_Black_C" 0 "NewEnumerator1"))
          (Math|Integer|IncrementInt (Variables|Default|GetChangeBlock)
            (:%20%20
              _)))
        (:1
          (Variables|Default|SetBlockChoise (Utilities|Struct|MakeBlockStruct "/Game/World/GridBlock/BluePrints/Block_Blue.Block_Blue_C" 0 "NewEnumerator2"))
          (Math|Integer|IncrementInt (Variables|Default|GetChangeBlock)
            (:%20%20
              _)))
        (:2
          (Variables|Default|SetBlockChoise (Utilities|Struct|MakeBlockStruct "/Game/World/GridBlock/BluePrints/Block_BASE.Block_BASE_C" 0 "NewEnumerator2"))
          (Math|Integer|IncrementInt (Variables|Default|GetChangeBlock)
            (:%20%20
              _))))
      (bind _pos (Default|GetGridPos (.actorblock (Variables|Default|GetBlockChoise)) (.type (Variables|Default|GetBlockChoise))))
      (bind _returnvalue (Game|SpawnActorfromClass (.blockclass (Variables|Default|GetBlockChoise)) (Math|Conversions|ToTransform(Vector) _pos) "Undefined" 0 0))
      (bind _output_get_2 (Variables|Default|SetBlockChoise (Utilities|Struct|MakeBlockStruct (.blockclass (Variables|Default|GetBlockChoise)) _returnvalue (.type (Variables|Default|GetBlockChoise)))))
      (bind _returnvalue_2 (Rendering|Material|CreateDynamicMaterialInstance (Variables|/Game/World/GridBlock/BluePrints/Block_BASE.Block_BASE_C|GetMat (.actorblock _output_get_2)) "None" :!class /Script/Engine.KismetMaterialLibrary))
      (Rendering|Material|SetScalarParameterValue _returnvalue_2 "MyOpacity" 0.5 :!class /Script/Engine.MaterialInstanceDynamic)
      (Rendering|Material|SetMaterial (Variables|/Game/World/GridBlock/BluePrints/Block_BASE.Block_BASE_C|GetCube (.actorblock _output_get_2)) 0 _returnvalue_2)
      (else
        (Actor|DestroyActor (.actorblock (Variables|Default|GetBlockChoise)))))))

(event Input|MouseEvents|RightMouseButton
  (params (Key :type Key%20Structure :default "None"))
  (bind _blockchoise (Variables|Default|GetBlockChoise))
  (bind _cube (Variables|Default|GetCube))
  (bind _returnvalue (Transformation|GetWorldLocation _cube))
  ;[0 0 0] Spawn Block
  (:Pressed
    (if (Variables|Default|GetBuildSystem)
      (bind (_pos _rotation) (Default|GetGridPos (.actorblock _blockchoise) (.type _blockchoise)))
      (if (<= (Math|Vector|Distance(Vector) _pos _returnvalue) (Variables|Default|GetDistanceToSpawnBlock))
        (bind _returnvalue_2 (Collision|LineTraceByChannel _returnvalue (Math|Vector|GetForwardVector (Math|Conversions|RotationFromXVector _pos)) "TraceTypeQuery1" false 0 "None"))
        (if _returnvalue_2
          (if (not (Variables|/Game/World/GridBlock/BluePrints/Block_BASE.Block_BASE_C|GetHitSomethings (.actorblock (Variables|Default|GetBlockChoise))))
            (Game|SpawnActorfromClass (.blockclass _blockchoise) (Math|Transform|MakeTransform _pos _rotation "1,1,1") "Undefined" 0 0)))))))

(event Input|MouseEvents|MouseWheelUp
  (params (Key :type Key%20Structure :default "None"))
  ;[0 0 0] Zoom/Dezoom
  (:Pressed
    (Default|Zoom (Variables|Default|GetCamera))))

(event Input|MouseEvents|MouseWheelDown
  (params (Key :type Key%20Structure :default "None"))
  ;[0 0 0] Zoom/Dezoom
  (:Pressed
    (Default|Dezoom (Variables|Default|GetCamera))))

(fn ConstructionScript)