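; Base Blueprint for a clickable resource block that the player works to harvest items.
; Hovering highlights the mesh through custom depth, and left-clicking stores the block as the character's SelectionUseBlock.
; When the player enters the collider of the selected block, the character works for a random delay.
; The block then spawns a random number of its item class between two marker positions and destroys itself.
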(event OnComponentBeginOverlap(Collider)
  (params (OverlappedComponent :type Primitive%20Component%20Object%20Reference) (OtherActor :type Actor%20Object%20Reference) (OtherComp :type Primitive%20Component%20Object%20Reference) (OtherBodyIndex :type Integer) (bFromSweep :type Boolean) (SweepResult :type Hit%20Result%20Structure%20%28by%20ref%29))
  (bind _returnvalue (Game|GetPlayerCharacter 0))
  (bind _asbp_character (Utilities|Casting|CastToBP_Character _returnvalue))
  (if (== OtherActor (Game|GetPlayerCharacter 0))
    (Variables|Default|SetPlayerIsIn true)
    (if (== (Variables|/Game/Player/Blueprints/BP_Character.BP_Character_C|GetSelectionUseBlock _asbp_character) self)
      (Development|PrintString "Work")
      (Default|Work _asbp_character)
      (Utilities|FlowControl|Delay (Math|Random|RandomFloatinRange 2.0 7.0))
      (Default|EndWork _asbp_character)
      (CallFunction|DestroyRessource))))

(event OnComponentEndOverlap(Collider)
  (params (OverlappedComponent :type Primitive%20Component%20Object%20Reference) (OtherActor :type Actor%20Object%20Reference) (OtherComp :type Primitive%20Component%20Object%20Reference) (OtherBodyIndex :type Integer))
  (if (== OtherActor (Game|GetPlayerCharacter 0))
    (Variables|Default|SetPlayerIsIn false)))

(event OnBeginCursorOver(Mesh)
  (params (TouchedComponent :type Primitive%20Component%20Object%20Reference))
  (CallFunction|HighLight true))

(event OnEndCursorOver(Mesh)
  (params (TouchedComponent :type Primitive%20Component%20Object%20Reference))
  (CallFunction|HighLight false))

(event OnClicked(Mesh)
  (params (TouchedComponent :type Primitive%20Component%20Object%20Reference) (ButtonPressed :type Key%20Structure :default "None"))
  (if (== ButtonPressed "LeftMouseButton")
    (Variables|/Game/Player/Blueprints/BP_Character.BP_Character_C|SetSelectionUseBlock (.AsBP%20Character (Utilities|Casting|CastToBP_Character (Game|GetPlayerCharacter 0))) self)))

(event Custom|HighLight
  (params (Active/Desactive :type Boolean))
  (Rendering|SetRenderCustomDepth (Variables|Default|GetMesh) Active/Desactive))

(event Custom|DestroyRessource
  (bind _minmaxressource (Variables|Default|GetMinMaxRessource))
  (bind _minpos (Variables|Default|GetMinPos))
  (bind _maxpos (Variables|Default|GetMaxPos))
  (bind _returnvalue (Transformation|GetWorldLocation _maxpos))
  (bind _returnvalue_2 (Transformation|GetWorldLocation _minpos))
  (for _index (range 0 (Math|Random|RandomIntegerinRange (Math|Float|Truncate (.x _minmaxressource)) (Math|Float|Truncate (.y _minmaxressource))))
    (Game|SpawnActorfromClass (.classitem (Variables|Default|GetItem)) (Math|Transform|MakeTransform (Math|Vector|MakeVector (Math|Random|RandomFloatinRange (.x _returnvalue_2) (.x _returnvalue)) (Math|Random|RandomFloatinRange (.y _returnvalue_2) (.y _returnvalue)) (Math|Random|RandomFloatinRange (.z _returnvalue_2) (.z _returnvalue))) "0, 0, 0" "1,1,1") "Undefined" 0 0)
    (Variables|Default|SetPlayerIsIn false))
  (Actor|DestroyActor))

(event EventBeginPlay)

(event Collision|EventActorBeginOverlap
  (params (OtherActor :type Actor%20Object%20Reference)))

(event EventTick
  (params (DeltaSeconds :type Float%20%28single-precision%29)))

(fn ConstructionScript)