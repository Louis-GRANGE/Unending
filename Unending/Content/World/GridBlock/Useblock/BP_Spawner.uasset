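; Resource spawner that scatters actors of a configurable class over a square area at Z=0 on BeginPlay, only when the game instance flags a first save.
; Random positions are re-rolled when too close to the previously spawned actors it checks, until the target count is reached.
; The retry counter is incremented but never caps the loop.
; The spawned array is then stored in General_Instance and the first-save flag is cleared.
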(event EventBeginPlay
  (bind _asgeneral_instance (Utilities|Casting|CastToGeneral_Instance (Game|GetGameInstance)))
  (if (Variables|/Game/UI/MainMenu/General_Instance.General_Instance_C|GetisFirstSave _asgeneral_instance)
    (bind (_posxout _posyout) (CallFunction|GenerateRandomVector))
    (bind _output_get (Variables|Default|SetMemVector (Math|Vector|MakeVector _posxout _posyout 0.0)))
    (bind _returnvalue (Game|SpawnActorfromClass (Variables|Parameters|GetClassRefActorToSpawn) (Math|Transform|MakeTransform _output_get "0, 0, 0" "1,1,1") "Undefined" 0 0))
    (Utilities|Array|Add (Variables|Default|GetRessources_Array) _returnvalue)
    ;[1 0 0.2109] While not as ressources as we want
    (while (< (Utilities|Array|Length (Variables|Default|GetRessources_Array)) (Variables|Parameters|GetRessourcesToSpawn))
      (bind (_posxout_2 _posyout_2) (CallFunction|GenerateRandomVector))
      (Variables|Default|SetMemVector (Math|Vector|MakeVector _posxout_2 _posyout_2 0.0))
      (Variables|Default|Setindex 0)
      (while (< (Variables|Default|Getindex) (- (Utilities|Array|Length (Variables|Default|GetRessources_Array)) 1))
        (if (> (Math|Vector|Distance(Vector) (Variables|Default|GetMemVector) (Transformation|GetWorldLocation (Variables|/Script/Engine.Actor|GetRootComponent (Utilities|Array|Get(acopy) (Variables|Default|GetRessources_Array) (Variables|Default|Getindex))))) (Variables|Parameters|GetOffest))
          (Math|Integer|IncrementInt (Variables|Default|Getindex)
            (:%20%20
              (if true
                _)))
          (else
            (bind (_posxout_3 _posyout_3) (CallFunction|GenerateRandomVector))
            (Variables|Default|SetMemVector (Math|Vector|MakeVector _posxout_3 _posyout_3 0.0))
            (Variables|Default|Setindex 0)
            (Math|Integer|IncrementInt (Variables|Default|GetInifiniteSecurity)))))
      ;[0 1 0.1328] SpawnActor
      (bind _returnvalue_2 (Game|SpawnActorfromClass (Variables|Parameters|GetClassRefActorToSpawn) (Math|Transform|MakeTransform (Variables|Default|GetMemVector) "0, 0, 0" "1,1,1") "Undefined" 0 0))
      (Utilities|Array|Add (Variables|Default|GetRessources_Array) _returnvalue_2))
    (bind _asgeneral_instance_2 (Utilities|Casting|CastToGeneral_Instance (Game|GetGameInstance)))
    (Variables|/Game/UI/MainMenu/General_Instance.General_Instance_C|SetisFirstSave _asgeneral_instance_2 false)
    (Variables|/Game/UI/MainMenu/General_Instance.General_Instance_C|SetRessourceArray _asgeneral_instance_2 (Variables|Default|GetRessources_Array))))

(fn ConstructionScript)

(fn GenerateRandomVector
  (bind _maxrangetospawn (Variables|Parameters|GetMaxRangeToSpawn))
  (LocalVariables|SetPosX (Math|Random|RandomFloatinRange 0.0 _maxrangetospawn))
  (LocalVariables|SetPosY (Math|Random|RandomFloatinRange 0.0 _maxrangetospawn))
  (return (LocalVariables|GetPosX) (LocalVariables|GetPosY)))