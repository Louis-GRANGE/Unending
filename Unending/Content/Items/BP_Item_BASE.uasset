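; BP_Item_BASE is a pickup item, named as a base class, that adds itself to the player's inventory on touch.
; When its Collider overlaps player character 0, it searches the BP_Character Inventory for an entry matching its ItemInfo Type.
; A match has its quantity increased by the item's quantity; otherwise ItemInfo is appended as a new entry.
; The actor destroys itself in either case.
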(event OnComponentBeginOverlap(Collider)
  (params (OverlappedComponent :type Primitive%20Component%20Object%20Reference) (OtherActor :type Actor%20Object%20Reference) (OtherComp :type Primitive%20Component%20Object%20Reference) (OtherBodyIndex :type Integer) (bFromSweep :type Boolean) (SweepResult :type Hit%20Result%20Structure%20%28by%20ref%29))
  (bind _returnvalue (Game|GetPlayerCharacter 0))
  (bind _iteminfo (Variables|Default|GetitemInfo))
  (bind _asbp_character (Utilities|Casting|CastToBP_Character _returnvalue))
  (bind _inventory (Variables|/Game/Player/Blueprints/BP_Character.BP_Character_C|GetInventory _asbp_character))
  (bind _returnvalue_2 (Utilities|Array|Length _inventory))
  (if (== OtherActor _returnvalue)
    (if (> _returnvalue_2 0)
      _
      (else
        _))
    (bind _index (Utilities|FlowControl|ForLoopwithBreak 0 (- _returnvalue_2 1) :!label _label)
      (:LoopBody
        (if (== (.type (Utilities|Array|Get(acopy) _inventory _index)) (.type _iteminfo))
          (Utilities|Array|SetArrayElem _inventory _index (Utilities|Struct|MakeStruct_ItemInfo (.classitem (Utilities|Array|Get(acopy) _inventory _index)) (.name (Utilities|Array|Get(acopy) _inventory _index)) (.type (Utilities|Array|Get(acopy) _inventory _index)) (+ (.quantity (Utilities|Array|Get(acopy) _inventory _index)) (.quantity _iteminfo))))
          (Variables|Default|SetIsInInventory true)
          (Actor|DestroyActor)
          (goto _label Break)))
      (:Completed
        (if (not (Variables|Default|GetIsInInventory))
          (Utilities|Array|Add _inventory (Variables|Default|GetitemInfo))
          (Actor|DestroyActor))))))

(event EventBeginPlay)

(event Collision|EventActorBeginOverlap
  (params (OtherActor :type Actor%20Object%20Reference)))

(event EventTick
  (params (DeltaSeconds :type Float%20%28single-precision%29)))

(fn ConstructionScript)